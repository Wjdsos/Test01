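; BP_PlayerState holds the player's current and max HP for the Survival game and exposes damage, heal and death-check functions.
; AddDamage and AddHeal change CurHP without clamping, then broadcast UpdateHP with current and max values so listeners can react.
; AddDamage also fires UpdateDeath whenever HP is below 1, the same threshold IsDeath returns, with no guard against repeat broadcasts.
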(fn `AddDamage`
  (params (Damage :type "Float (double-precision)"))
  (bind _output_get (set `self.CurHP` (- (`self.CurHP`) Damage)))
  (`self.EventDispatcherUpdateHP` _output_get (`self.MaxHP`))
  (if (< (`self.CurHP`) 1.0)
    (`self.EventDispatcherUpdateDeath`)))

(fn `AddHeal`
  (params (Heal :type "Float (double-precision)"))
  (bind _output_get (set `self.CurHP` (+ (`self.CurHP`) Heal)))
  (`self.EventDispatcherUpdateHP` _output_get (`self.MaxHP`)))

(fn `IsDeath`
  (returns (IsDeath :type Boolean))
  (return (< (`self.CurHP`) 1.0)))

(fn `UserConstructionScript`)